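; DynamicPlaceholder01 is an actor Blueprint that oscillates back and forth along world X.
; Each Tick adds a world offset from a sine of game time, scaled by delta seconds and Distance, so Distance sets peak speed and Frequency the rate.
; BeginPlay picks a random time offset, scaled by Frequency, to vary each instance's phase.
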(event `self.ReceiveBeginPlay`
  (set `self.RandStart` (/ (`KismetMathLibrary.RandomFloat`) (`self.Frequency`))))

(event `self.ReceiveTick`
  (params (DeltaSeconds :type "Float (single-precision)"))
  (`self.K2_AddActorWorldOffset` (`KismetMathLibrary.MakeVector` (* (* DeltaSeconds (`self.Distance`)) (`KismetMathLibrary.Sin` (* (* (+ (`KismetSystemLibrary.GetGameTimeInSeconds`) (`self.RandStart`)) (`self.Frequency`)) 3.141593))))))

(fn `UserConstructionScript`)