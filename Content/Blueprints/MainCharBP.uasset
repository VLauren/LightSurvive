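; MainCharBP is the player character, with axis-driven movement and look and a point light that continuously pulses.
; Move inputs follow control-rotation yaw only, while look inputs feed controller yaw and pitch.
; Tick runs a ping-pong counter between negative OffTime and LightTime, scaling light intensity linearly from it.
; The counter's dip below zero gives negative intensity values, apparently intended as a dark interval between pulses.
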(event `self.ReceiveTick`
  (params (DeltaSeconds :type "Float (single-precision)"))
  (bind _lightcounter (`self.LightCounter`))
  (set `self.LightCounter` (select `bool` (`self.IncreaseLight`) :`false` (- _lightcounter DeltaSeconds) :`true` (+ _lightcounter DeltaSeconds)))
  (`LightComponent.SetIntensity` (`self.PointLight`) (* (`self.LightIntensity`) (/ (`self.LightCounter`) (`self.LightTime`))))
  (if (or (and (> (`self.LightCounter`) (`self.LightTime`)) (`self.IncreaseLight`)) (and (< (`self.LightCounter`) (* (`self.OffTime`) -1.0)) (not (`self.IncreaseLight`))))
    (set `self.IncreaseLight` (not (`self.IncreaseLight`)))))

(event `InputAxis|MoveForward`
  (params (AxisValue :type "Float (single-precision)"))
  (`self.AddMovementInput` (`KismetMathLibrary.GetForwardVector` (`KismetMathLibrary.MakeRotator` 0.0 0.0 (.yaw (`self.GetControlRotation`)))) AxisValue))

(event `InputAxis|MoveRight`
  (params (AxisValue :type "Float (single-precision)"))
  (`self.AddMovementInput` (`KismetMathLibrary.GetRightVector` (`KismetMathLibrary.MakeRotator` 0.0 0.0 (.yaw (`self.GetControlRotation`)))) AxisValue))

(event `InputAxis|LookRight`
  (params (AxisValue :type "Float (single-precision)"))
  (`self.AddControllerYawInput` AxisValue))

(event `InputAxis|LookUp`
  (params (AxisValue :type "Float (single-precision)"))
  (`self.AddControllerPitchInput` AxisValue))

(fn `UserConstructionScript`)